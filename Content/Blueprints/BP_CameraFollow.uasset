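; Side-scrolling follow camera that tracks the WatchPoint of the platformer character.
; CamInitialize places the camera CamStartDist along the character's right vector and aims it at the WatchPoint once, using GetRotationToTarget.
; Tick then eases world X and Z toward the WatchPoint at separate horizontal and vertical speeds, leaving Y and rotation untouched.
; Only initialization checks that the character reference is valid.
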(event `CamInitialize`
  (bind _bp_platformercharacter (`self.Bp_PlatformerCharacter`))
  (if (`KismetSystemLibrary.IsValid` (`self.Bp_PlatformerCharacter`))
    (`self.K2_SetActorLocation` (+ (`SceneComponent.K2_GetComponentLocation` (`/Game/Blueprints/BP_PlatformerCharacter.WatchPoint` _bp_platformercharacter)) (* (`SceneComponent.GetRightVector` (`Actor.RootComponent` _bp_platformercharacter)) (`self.CamStartDist`))))
    (`self.K2_SetActorRotation` (`self.GetRotationToTarget`))))

(event `self.ReceiveTick`
  (params (DeltaSeconds :type "Float (single-precision)"))
  (bind (_returnvalue_x _returnvalue_y) (`KismetMathLibrary.BreakVector` (`self.K2_GetActorLocation`)))
  (bind _returnvalue (`self.K2_GetActorLocation`))
  (bind (_returnvalue_x_2 _returnvalue_y_2 _returnvalue_z) (`KismetMathLibrary.BreakVector` (`self.K2_GetActorLocation`)))
  (bind (_returnvalue_x_3 _returnvalue_y_3 _returnvalue_z_2) (`KismetMathLibrary.BreakVector` (`SceneComponent.K2_GetComponentLocation` (`/Game/Blueprints/BP_PlatformerCharacter.WatchPoint` (`self.Bp_PlatformerCharacter`)))))
  (bind _returnvalue_x_4 (`KismetMathLibrary.BreakVector` (`SceneComponent.K2_GetComponentLocation` (`/Game/Blueprints/BP_PlatformerCharacter.WatchPoint` (`self.Bp_PlatformerCharacter`)))))
  (`self.K2_SetActorLocation` (`KismetMathLibrary.VInterpTo` _returnvalue (`KismetMathLibrary.MakeVector` _returnvalue_x_4 _returnvalue_y_2 _returnvalue_z) DeltaSeconds (`self.Interp Speed Left Right`)))
  (`self.K2_SetActorLocation` (`KismetMathLibrary.VInterpTo` _returnvalue (`KismetMathLibrary.MakeVector` _returnvalue_x _returnvalue_y _returnvalue_z_2) DeltaSeconds (`self.Interp Speed Up Down`))))

(fn `GetRotationToTarget`
  (returns (ReturnValue :type "Rotator Structure"))
  (return (`KismetMathLibrary.MakeRotFromX` (`KismetMathLibrary.Normal` (- (`SceneComponent.K2_GetComponentLocation` (`/Game/Blueprints/BP_PlatformerCharacter.WatchPoint` (`self.Bp_PlatformerCharacter`))) (`SceneComponent.K2_GetComponentLocation` (`self.Camera`)))))))

(fn `UserConstructionScript`)