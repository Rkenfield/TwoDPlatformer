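; BP_GrapplePointSwing is a swing grapple point that registers itself with the platformer character's Grapple component when the character comes within range.
; The construction script sizes its trigger sphere to one and a half times MaxRestLen.
; Entering sets it as the swing point unless the character is already grappled, with a debug print.
; Leaving clears it if still current, then ends and detaches the grapple.
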(event `self.Sphere1.OnComponentBeginOverlap`
  (params (OverlappedComponent :type "PrimitiveComponent Object Reference") (OtherActor :type "Actor Object Reference") (OtherComp :type "PrimitiveComponent Object Reference") (OtherBodyIndex :type Integer) (bFromSweep :type Boolean) (SweepResult :type "HitResult Structure (by ref)"))
  (bind _asbp_platformer_character (cast `/Game/Blueprints/BP_PlatformerCharacter` OtherActor))
  (bind _grapple (`/Game/Blueprints/BP_PlatformerCharacter.Grapple` _asbp_platformer_character))
  (if (not (`GrappleComponent.IsGrappled` _grapple))
    (set `GrappleComponent.GrapplePointSwing` self _grapple)
    (`KismetSystemLibrary.PrintString` "Set Grapple point")))

(event `self.Sphere1.OnComponentEndOverlap`
  (params (OverlappedComponent :type "PrimitiveComponent Object Reference") (OtherActor :type "Actor Object Reference") (OtherComp :type "PrimitiveComponent Object Reference") (OtherBodyIndex :type Integer))
  (bind _asbp_platformer_character (cast `/Game/Blueprints/BP_PlatformerCharacter` OtherActor))
  (bind _grapple (`/Game/Blueprints/BP_PlatformerCharacter.Grapple` _asbp_platformer_character))
  (if (== self (`GrappleComponent.GrapplePointSwing` _grapple))
    (set `GrappleComponent.GrapplePointSwing` null _grapple)
    (`GrappleComponent.EndGrapple` _grapple)
    (`/Game/Blueprints/BP_PlatformerCharacter.DetachGrapple` _asbp_platformer_character)))

(fn `UserConstructionScript`
  (`SphereComponent.SetSphereRadius` (`self.Sphere1`) (* (`self.MaxRestLen`) 1.5) true))